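; BP_Branch is a node of a recursively spawned binary tree, built as a Composite pattern with leaf actors at the ends.
; On BeginPlay it spawns left and right child branches at NextBranchesRoot until MaxHierarchyLevel, then spawns BP_Leaf actors instead.
; Children shrink in scale and roll to opposite sides by an angle that decays exponentially with depth.
; GetSum recursively adds the results of both children.
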(event `self.ReceiveBeginPlay`
  (set `self.DeltaRotationX` (* 90.0 (`KismetMathLibrary.MultiplyMultiply_FloatFloat` 0.6 (`KismetMathLibrary.Conv_IntToDouble` (`self.HierarchyLevel`)))))
  (if (< (`self.HierarchyLevel`) (`self.MaxHierarchyLevel`))
    (bind _result (`self.Spawn Branch` true))
    (set `self.LeftBranch` _result)
    (bind _result_2 (`self.Spawn Branch` false))
    (set `self.RightBranch` _result_2)
    (else
      (bind _result_3 (`self.Spawn Leaf` true))
      (set `self.LeftBranch` _result_3)
      (bind _result_4 (`self.Spawn Leaf` false))
      (set `self.RightBranch` _result_4))))

(fn `GetSum`
  (returns (ReturnValue :type Integer))
  (bind _returnvalue (`Summable.GetSum` (`self.LeftBranch`)))
  (bind _returnvalue_2 (`Summable.GetSum` (`self.RightBranch`)))
  (return (+ _returnvalue_2 _returnvalue)))

(fn `Spawn Branch`
  (params (IsLeft :type Boolean))
  (returns (Result :type "Summable Interface"))
  (bind (_returnvalue_roll _returnvalue_pitch _returnvalue_yaw) (`KismetMathLibrary.BreakRotator` (`SceneComponent.K2_GetComponentRotation` (`self.DefaultSceneRoot`))))
  (bind _returnvalue (`|SpawnActorFromClass` "BP_Branch_C" (`KismetMathLibrary.MakeTransform` (`SceneComponent.K2_GetComponentLocation` (`self.NextBranchesRoot`)) (`KismetMathLibrary.MakeRotator` (+ (* (`KismetMathLibrary.SelectInt` 1 -1 IsLeft) (`self.DeltaRotationX`)) _returnvalue_roll) _returnvalue_pitch _returnvalue_yaw) (* (`SceneComponent.K2_GetComponentScale` (`self.DefaultSceneRoot`)) 0.9)) "Undefined" "OverrideRootScale" null 0.0 (+ (`self.HierarchyLevel`) 1) (`self.MaxHierarchyLevel`) null))
  (return _returnvalue))

(fn `Spawn Leaf`
  (params (IsLeft :type Boolean))
  (returns (Result :type "Summable Interface"))
  (bind (_returnvalue_roll _returnvalue_pitch _returnvalue_yaw) (`KismetMathLibrary.BreakRotator` (`SceneComponent.K2_GetComponentRotation` (`self.DefaultSceneRoot`))))
  (bind _returnvalue (`|SpawnActorFromClass` "/Game/Blueprints/Composite/BP_Leaf.BP_Leaf_C" (`KismetMathLibrary.MakeTransform` (`SceneComponent.K2_GetComponentLocation` (`self.NextBranchesRoot`)) (`KismetMathLibrary.MakeRotator` (+ (* (`KismetMathLibrary.SelectInt` 1 -1 IsLeft) (`self.DeltaRotationX`)) _returnvalue_roll) _returnvalue_pitch _returnvalue_yaw) (* (`SceneComponent.K2_GetComponentScale` (`self.DefaultSceneRoot`)) 0.9)) "Undefined" "OverrideRootScale" null null))
  (return _returnvalue))

(fn `UserConstructionScript`)